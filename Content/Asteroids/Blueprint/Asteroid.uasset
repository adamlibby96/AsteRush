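; Destructible asteroid actor that loses health from TwinStickProjectile hits, destroying each projectile on impact.
; Tick polls health on the authority: at zero or below, big asteroids split into smaller-tier ones and others scatter Money pickups, then destroy themselves.
; SpawnBabyAsteroids spawns a random count around the parent using randomized transforms, skipping colliding spawns.
; A CanSpawnBabies flag gates the parent's destruction until spawning completes.
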(event EventTick
  (params (DeltaSeconds :type Float%20%28single-precision%29))
  (Networking|SwitchHasAuthority
    (:Authority
      (if (<= (Variables|Default|GetHealth) 0.0)
        (if (Variables|Default|GetisBigAsteroid)
          (CallFunction|SpawnBabyAsteroids (Transformation|GetWorldTransform (Variables|Default|GetAsteroid1)) (Variables|Default|GetBabyAste_RotAngle) (Variables|Default|GetBabyAste_MinScale) (Variables|Default|GetBabyAste_MaxScale) (Variables|Default|GetBabyAste_MaxNumToSpawn) (Variables|Default|GetBabyAste_MinNumtoSpawn))
          (while (not (Variables|Default|GetcanSpawnBabies))
            _)
          (Actor|DestroyActor)
          (else
            (CallFunction|DropLoot 10 (Transformation|GetWorldLocation (Variables|Default|GetAsteroid1)))
            (Actor|DestroyActor)))))))

(event Collision|EventHit
  (params (MyComp :type Primitive%20Component%20Object%20Reference) (Other :type Actor%20Object%20Reference) (OtherComp :type Primitive%20Component%20Object%20Reference) (bSelfMoved :type Boolean) (HitLocation :type Vector :default "0, 0, 0") (HitNormal :type Vector :default "0, 0, 0") (NormalImpulse :type Vector :default "0, 0, 0") (Hit :type Hit%20Result%20Structure%20%28by%20ref%29))
  (bind _astwin_stick_projectile (Utilities|Casting|CastToTwinStickProjectile Other))
  (Variables|Default|SetHealth (- (Variables|Default|GetHealth) (Variables|/Game/TwinStickBP/Blueprints/TwinStickProjectile.TwinStickProjectile_C|GetDamage _astwin_stick_projectile)))
  (Actor|DestroyActor _astwin_stick_projectile))

(fn ConstructionScript)

(fn DropLoot
  (params (AmountOfLoot :type Integer) (InitialLocation :type Vector))
  (bind _coinspawnrange (Variables|Default|GetCoinSpawnRange))
  (for _index (range 0 AmountOfLoot)
    (Networking|SwitchHasAuthority
      (:Authority
        (Game|SpawnActorfromClass "/Game/TwinStickBP/Blueprints/Money.Money_C" (Math|Transform|MakeTransform (Math|Vector|MakeVector (Math|Random|RandomFloatinRange (- (.x InitialLocation) _coinspawnrange) (+ (.x InitialLocation) _coinspawnrange)) (Math|Random|RandomFloatinRange (- (.y InitialLocation) _coinspawnrange) (+ (.y InitialLocation) _coinspawnrange)) 0.0) "0, 0, 0" "1,1,1") "AdjustIfPossibleButAlwaysSpawn" 0 0)))))

(fn SpawnBabyAsteroids
  (params (StartTransform :type Transform) (RandomRotAngle :type Float%20%28single-precision%29) (Minscale :type Float%20%28single-precision%29) (Maxscale :type Float%20%28single-precision%29) (MaxNumToSpawn :type Integer) (MinNumToSpawn :type Integer))
  (Utilities|FlowControl|Sequence
    (:then_0
      ;[1 1 1] Setup local variables
      (LocalVariables|SetStartingLocation StartTransform)
      (LocalVariables|SetSpawn%20Radius (Variables|Default|GetBabyAsteroidRange))
      (LocalVariables|SetRandom%20Rotation%20Angle RandomRotAngle)
      (LocalVariables|SetMinScaleSize Minscale)
      (LocalVariables|SetMaxScaleSize Maxscale))
    (:then_1
      (Variables|Default|SetcanSpawnBabies false)
      (for _index (range 0 (Math|Random|RandomIntegerinRange MinNumToSpawn MaxNumToSpawn))
        (bind _returnvalue (Game|SpawnActorfromClass "Asteroid_C" (Utilities|GetRandomTransform (Math|Transform|MakeTransform (Math|Vector|MakeVector (.x (.location (LocalVariables|GetStartingLocation))) (.y (.location (LocalVariables|GetStartingLocation))) 0.0) (.rotation (LocalVariables|GetStartingLocation))) (LocalVariables|GetSpawn%20Radius) (LocalVariables|GetRandom%20Rotation%20Angle) (LocalVariables|GetMinScaleSize) (LocalVariables|GetMaxScaleSize)) "AdjustIfPossibleButDontSpawnIfColliding" 0 0))
        (Variables|Asteroid_C|SetisBigAsteroid _returnvalue false))
      (Variables|Default|SetcanSpawnBabies true))))